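; Spear projectile tied to a Player ID that ends the round when it hits a character with a different PawnID.
; Once SpearMovement is called, it travels along +X for player 0 or -X otherwise, chaining timeline-driven 200-unit lerps indefinitely by restarting from its new location.
; A box overlap with an opposing Player1_Character reports the winner and hit component to PlayerGameMode's NewRound, then destroys the spear.
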(event OnComponentBeginOverlap(Box)
  (params (OverlappedComponent :type Primitive%20Component%20Object%20Reference) (OtherActor :type Actor%20Object%20Reference) (OtherComp :type Primitive%20Component%20Object%20Reference) (OtherBodyIndex :type Integer) (bFromSweep :type Boolean) (SweepResult :type Hit%20Result%20Structure%20%28by%20ref%29))
  (bind _asplayer_1_character (Utilities|Casting|CastToPlayer1_Character OtherActor))
  (if (not (== (Variables|/Game/JamStadium/Player1_Character.Player1_Character_C|GetPawnID _asplayer_1_character) (Variables|Default|GetPlayer)))
    (Default|NewRound (.AsPlayer%20Game%20Mode (Utilities|Casting|CastToPlayerGameMode (Game|GetGameMode))) (Variables|Default|GetPlayer) (Transformation|GetWorldLocation OtherComp) OtherComp)
    (Actor|DestroyActor)))

(event Custom|SpearMovement
  (if (== (Variables|Default|GetPlayer) 0)
    (Variables|Default|SetInitialLocation (Transformation|GetActorLocation) :!label _label)
    (bind _float (Timeline|Speed PlayFromStart)
      (:Update
        (Transformation|SetActorLocation (Math|Vector|Lerp(Vector) (Variables|Default|GetInitialLocation) (Math|Vector|MakeVector (+ (.x (Variables|Default|GetInitialLocation)) 2e+02) (.y (Variables|Default|GetInitialLocation)) (.z (Variables|Default|GetInitialLocation))) _float) false false))
      (:Finished
        (goto _label)))
    (else
      (Variables|Default|SetInitialLocation (Transformation|GetActorLocation) :!label _label_2)
      (bind _float_2 (Timeline|Timeline_1 PlayFromStart)
        (:Update
          (Transformation|SetActorLocation (Math|Vector|Lerp(Vector) (Variables|Default|GetInitialLocation) (Math|Vector|MakeVector (- (.x (Variables|Default|GetInitialLocation)) 2e+02) (.y (Variables|Default|GetInitialLocation)) (.z (Variables|Default|GetInitialLocation))) _float_2) false false))
        (:Finished
          (goto _label_2))))))

(event EventBeginPlay)

(event Collision|EventActorBeginOverlap
  (params (OtherActor :type Actor%20Object%20Reference)))

(event EventTick
  (params (DeltaSeconds :type Float%20%28single-precision%29)))

(fn ConstructionScript)
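; Main menu and two-player character selection screen for JamStadium, switching from menu to selection by toggling component visibility.
; Externally triggered left, right and select events move a robot marker between menu options or each player's blue or yellow spotlight across four characters.
; Confirming whitens the spotlight and stores the choice in CustomGameInstance; only player 1 has a cancel.
; Once both confirm, it removes the second player and opens LevelTest.
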(event Custom|P2SelectionGoRight
  (Utilities|FlowControl|Sequence
    (:then_0
      (if (== (Variables|Default|GetP2Highlight) 1)
        (Rendering|Components|Light|SetIntensity (Variables|Default|GetYellowSpotLight1) 0.0)
        (Rendering|Components|Light|SetIntensity (Variables|Default|GetYellowSpotLight2) (Variables|Default|GetLightIntensity))))
    (:then_1
      (if (== (Variables|Default|GetP2Highlight) 2)
        (Rendering|Components|Light|SetIntensity (Variables|Default|GetYellowSpotLight2) 0.0)
        (Rendering|Components|Light|SetIntensity (Variables|Default|GetYellowSpotLight3) (Variables|Default|GetLightIntensity))))
    (:then_2
      (if (== (Variables|Default|GetP2Highlight) 3)
        (Rendering|Components|Light|SetIntensity (Variables|Default|GetYellowSpotLight3) 0.0)
        (Rendering|Components|Light|SetIntensity (Variables|Default|GetYellowSpotLight4) (Variables|Default|GetLightIntensity))))
    (:then_3
      (if (< (Variables|Default|GetP2Highlight) 4)
        (Variables|Default|SetP2Highlight (+ (Variables|Default|GetP2Highlight) 1))))))

(event Custom|SelectP2Character
  (Utilities|FlowControl|Sequence
    (:then_0
      (if (== (Variables|Default|GetP2Highlight) 1)
        (Variables|/Game/JamStadium/CustomGameInstance.CustomGameInstance_C|SetP2CharacterChoice (.AsCustom%20Game%20Instance (Utilities|Casting|CastToCustomGameInstance (Game|GetGameInstance))) 1)
        (Rendering|Components|Light|SetLightColor (Variables|Default|GetYellowSpotLight1) "(R=1.000000,G=1.000000,B=1.000000,A=1.000000)" true)
        (Variables|Default|SetP2Validation true :!label _label)
        (if (and (Variables|Default|GetP1Validation) (Variables|Default|GetP2Validation))
          (Class|GameplayStatics|RemovePlayer (Game|GetPlayerController 1) true)
          (Game|OpenLevel(byName) "LevelTest"))))
    (:then_1
      (if (== (Variables|Default|GetP2Highlight) 2)
        (Variables|/Game/JamStadium/CustomGameInstance.CustomGameInstance_C|SetP2CharacterChoice (.AsCustom%20Game%20Instance (Utilities|Casting|CastToCustomGameInstance (Game|GetGameInstance))) 2)
        (Rendering|Components|Light|SetLightColor (Variables|Default|GetYellowSpotLight2) "(R=1.000000,G=1.000000,B=1.000000,A=1.000000)" true)
        (goto _label)))
    (:then_2
      (if (== (Variables|Default|GetP2Highlight) 3)
        (Variables|/Game/JamStadium/CustomGameInstance.CustomGameInstance_C|SetP2CharacterChoice (.AsCustom%20Game%20Instance (Utilities|Casting|CastToCustomGameInstance (Game|GetGameInstance))) 3)
        (Rendering|Components|Light|SetLightColor (Variables|Default|GetYellowSpotLight3) "(R=1.000000,G=1.000000,B=1.000000,A=1.000000)" true)
        (goto _label)))
    (:then_3
      (if (== (Variables|Default|GetP2Highlight) 4)
        (Variables|/Game/JamStadium/CustomGameInstance.CustomGameInstance_C|SetP2CharacterChoice (.AsCustom%20Game%20Instance (Utilities|Casting|CastToCustomGameInstance (Game|GetGameInstance))) 4)
        (Rendering|Components|Light|SetLightColor (Variables|Default|GetYellowSpotLight4) "(R=1.000000,G=1.000000,B=1.000000,A=1.000000)" true)
        (goto _label)))))

(event Custom|P2SelectionGoLeft
  (Utilities|FlowControl|Sequence
    (:then_0
      (if (== (Variables|Default|GetP2Highlight) 4)
        (Rendering|Components|Light|SetIntensity (Variables|Default|GetYellowSpotLight4) 0.0)
        (Rendering|Components|Light|SetIntensity (Variables|Default|GetYellowSpotLight3) (Variables|Default|GetLightIntensity))))
    (:then_1
      (if (== (Variables|Default|GetP2Highlight) 3)
        (Rendering|Components|Light|SetIntensity (Variables|Default|GetYellowSpotLight3) 0.0)
        (Rendering|Components|Light|SetIntensity (Variables|Default|GetYellowSpotLight2) (Variables|Default|GetLightIntensity))))
    (:then_2
      (if (== (Variables|Default|GetP2Highlight) 2)
        (Rendering|Components|Light|SetIntensity (Variables|Default|GetYellowSpotLight2) 0.0)
        (Rendering|Components|Light|SetIntensity (Variables|Default|GetYellowSpotLight1) (Variables|Default|GetLightIntensity))))
    (:then_3
      (if (> (Variables|Default|GetP2Highlight) 1)
        (Variables|Default|SetP2Highlight (- (Variables|Default|GetP2Highlight) 1))))))

(event Custom|P1SelectionGoRight
  (Utilities|FlowControl|Sequence
    (:then_0
      (if (== (Variables|Default|GetP1Highlight) 1)
        (Rendering|Components|Light|SetIntensity (Variables|Default|GetBlueSpotLight1) 0.0)
        (Rendering|Components|Light|SetIntensity (Variables|Default|GetBlueSpotLight2) (Variables|Default|GetLightIntensity))))
    (:then_1
      (if (== (Variables|Default|GetP1Highlight) 2)
        (Rendering|Components|Light|SetIntensity (Variables|Default|GetBlueSpotLight2) 0.0)
        (Rendering|Components|Light|SetIntensity (Variables|Default|GetBlueSpotLight3) (Variables|Default|GetLightIntensity))))
    (:then_2
      (if (== (Variables|Default|GetP1Highlight) 3)
        (Rendering|Components|Light|SetIntensity (Variables|Default|GetBlueSpotLight3) 0.0)
        (Rendering|Components|Light|SetIntensity (Variables|Default|GetBlueSpotLight4) (Variables|Default|GetLightIntensity))))
    (:then_3
      (if (< (Variables|Default|GetP1Highlight) 4)
        (Variables|Default|SetP1Highlight (+ (Variables|Default|GetP1Highlight) 1))))))

(event Custom|SelectRight
  (params (Player :type Integer))
  ;[0 0.1451 1] PLAYER 1
  ;;[1 1 1] PLAYER 1 GO RIGHT
  (Variables|Default|SetPlayer Player)
  (if (Variables|Default|GetMain)
    (CallFunction|MenuGoRight)
    (elif (Variables|Default|GetCharacterSelection)
      (if (== (Variables|Default|GetPlayer) 0)
        (if (not (Variables|Default|GetP1Validation))
          (CallFunction|P1SelectionGoRight))
        (elif (not (Variables|Default|GetP2Validation))
          (CallFunction|P2SelectionGoRight))))))

(event Custom|MenuGoRight
  (bind _plane2 (Variables|Default|GetPlane2))
  (bind _papersprite (Variables|Default|GetPaperSprite))
  (bind _returnvalue (Transformation|GetWorldLocation _plane2))
  (bind _returnvalue_2 (Transformation|GetWorldLocation _papersprite))
  (bind (_x _y _z) (Math|Vector|BreakVector _returnvalue_2))
  (bind (_x_2 _y_2 _z_2) (Math|Vector|BreakVector _returnvalue))
  (Utilities|FlowControl|Sequence
    (:then_0
      (if (== (Variables|Default|GetMenuHightLight) 1)
        (Transformation|SetWorldLocation (Variables|Default|GetBueRobot) (Math|Vector|MakeVector (- _x_2 5e+01) _y_2 (+ _z_2 1e+02)) false false)
        (Variables|Default|SetMenuHightLight (+ (Variables|Default|GetMenuHightLight) 1))))
    (:then_1
      (if (== (Variables|Default|GetMenuHightLight) 0)
        (Transformation|SetWorldLocation (Variables|Default|GetBueRobot) (Math|Vector|MakeVector (- _x 5e+01) _y (+ _z 1e+02)) false false)
        (Variables|Default|SetMenuHightLight (+ (Variables|Default|GetMenuHightLight) 1))))))

(event Custom|MenuGoLeft
  (bind _hifi (Variables|Default|GetHifi))
  (bind _papersprite (Variables|Default|GetPaperSprite))
  (bind _returnvalue (Transformation|GetWorldLocation _papersprite))
  (bind _returnvalue_2 (Transformation|GetWorldLocation _hifi))
  (bind (_x _y _z) (Math|Vector|BreakVector _returnvalue))
  (bind (_x_2 _y_2 _z_2) (Math|Vector|BreakVector _returnvalue_2))
  (Utilities|FlowControl|Sequence
    (:then_0
      (if (== (Variables|Default|GetMenuHightLight) 1)
        (Transformation|SetWorldLocation (Variables|Default|GetBueRobot) (Math|Vector|MakeVector (- _x_2 5e+01) _y_2 (+ _z_2 1e+02)) false false)
        (Variables|Default|SetMenuHightLight (- (Variables|Default|GetMenuHightLight) 1))))
    (:then_1
      (if (== (Variables|Default|GetMenuHightLight) 2)
        (Transformation|SetWorldLocation (Variables|Default|GetBueRobot) (Math|Vector|MakeVector (- _x 5e+01) _y (+ _z 1e+02)) false false)
        (Variables|Default|SetMenuHightLight (- (Variables|Default|GetMenuHightLight) 1))))))

(event Custom|SelectLeft
  (params (Player :type Integer))
  ;[0 0.1451 1] PLAYER 1
  ;;[1 1 1] PLAYER 1 GO LEFT
  (Variables|Default|SetPlayer Player)
  (if (Variables|Default|GetMain)
    (CallFunction|MenuGoLeft)
    (elif (Variables|Default|GetCharacterSelection)
      (if (== (Variables|Default|GetPlayer) 0)
        (if (not (Variables|Default|GetP1Validation))
          (CallFunction|P1SelectionGoLeft))
        (elif (not (Variables|Default|GetP2Validation))
          (CallFunction|P2SelectionGoLeft))))))

(event Custom|P1SelectionGoLeft
  (Utilities|FlowControl|Sequence
    (:then_0
      (if (== (Variables|Default|GetP1Highlight) 4)
        (Rendering|Components|Light|SetIntensity (Variables|Default|GetBlueSpotLight4) 0.0)
        (Rendering|Components|Light|SetIntensity (Variables|Default|GetBlueSpotLight3) (Variables|Default|GetLightIntensity))))
    (:then_1
      (if (== (Variables|Default|GetP1Highlight) 3)
        (Rendering|Components|Light|SetIntensity (Variables|Default|GetBlueSpotLight3) 0.0)
        (Rendering|Components|Light|SetIntensity (Variables|Default|GetBlueSpotLight2) (Variables|Default|GetLightIntensity))))
    (:then_2
      (if (== (Variables|Default|GetP1Highlight) 2)
        (Rendering|Components|Light|SetIntensity (Variables|Default|GetBlueSpotLight2) 0.0)
        (Rendering|Components|Light|SetIntensity (Variables|Default|GetBlueSpotLight1) (Variables|Default|GetLightIntensity))))
    (:then_3
      (if (> (Variables|Default|GetP1Highlight) 1)
        (Variables|Default|SetP1Highlight (- (Variables|Default|GetP1Highlight) 1))))))

(event Custom|MenuSelect
  (Utilities|FlowControl|Sequence
    (:then_0
      (if (== (Variables|Default|GetMenuHightLight) 0)
        _))
    (:then_1
      (if (== (Variables|Default|GetMenuHightLight) 1)
        (Rendering|SetVisibility (Components|GetChildrenComponents (Variables|Default|GetMainMenu) true) false false)
        (Rendering|SetVisibility (Components|GetChildrenComponents (Variables|Default|GetPlayerSelect) false) true false)
        (Variables|Default|SetMain false)
        (Variables|Default|SetCharacterSelection true)))
    (:then_2
      (if (== (Variables|Default|GetMenuHightLight) 2)
        (Game|QuitGame 0 "Quit")))))

(event Custom|Select
  (params (Player :type Integer))
  ;[0 0.1451 1] PLAYER 1
  ;;[1 1 1] PLAYER 1 SELECT
  (Variables|Default|SetPlayer Player)
  (if (Variables|Default|GetMain)
    (CallFunction|MenuSelect)
    (elif (Variables|Default|GetCharacterSelection)
      (if (== (Variables|Default|GetPlayer) 0)
        (CallFunction|SelectP1Character)
        (else
          (CallFunction|SelectP2Character))))))

(event Custom|SelectP1Character
  (Utilities|FlowControl|Sequence
    (:then_0
      (if (== (Variables|Default|GetP1Highlight) 1)
        (Variables|/Game/JamStadium/CustomGameInstance.CustomGameInstance_C|SetP1CharacterChoice (.AsCustom%20Game%20Instance (Utilities|Casting|CastToCustomGameInstance (Game|GetGameInstance))) 1)
        (Rendering|Components|Light|SetLightColor (Variables|Default|GetBlueSpotLight1) "(R=1.000000,G=1.000000,B=1.000000,A=1.000000)" true)
        (Variables|Default|SetP1Validation true :!label _label)
        (if (and (Variables|Default|GetP1Validation) (Variables|Default|GetP2Validation))
          (Class|GameplayStatics|RemovePlayer (Game|GetPlayerController 1) true)
          (Game|OpenLevel(byName) "LevelTest"))))
    (:then_1
      (if (== (Variables|Default|GetP1Highlight) 2)
        (Variables|/Game/JamStadium/CustomGameInstance.CustomGameInstance_C|SetP1CharacterChoice (.AsCustom%20Game%20Instance (Utilities|Casting|CastToCustomGameInstance (Game|GetGameInstance))) 2)
        (Rendering|Components|Light|SetLightColor (Variables|Default|GetBlueSpotLight2) "(R=1.000000,G=1.000000,B=1.000000,A=1.000000)" true)
        (goto _label)))
    (:then_2
      (if (== (Variables|Default|GetP1Highlight) 3)
        (Variables|/Game/JamStadium/CustomGameInstance.CustomGameInstance_C|SetP1CharacterChoice (.AsCustom%20Game%20Instance (Utilities|Casting|CastToCustomGameInstance (Game|GetGameInstance))) 3)
        (Rendering|Components|Light|SetLightColor (Variables|Default|GetBlueSpotLight3) "(R=1.000000,G=1.000000,B=1.000000,A=1.000000)" true)
        (goto _label)))
    (:then_3
      (if (== (Variables|Default|GetP1Highlight) 4)
        (Variables|/Game/JamStadium/CustomGameInstance.CustomGameInstance_C|SetP1CharacterChoice (.AsCustom%20Game%20Instance (Utilities|Casting|CastToCustomGameInstance (Game|GetGameInstance))) 4)
        (Rendering|Components|Light|SetLightColor (Variables|Default|GetBlueSpotLight4) "(R=1.000000,G=1.000000,B=1.000000,A=1.000000)" true)
        (goto _label)))))

(event EventBeginPlay
  (Input|EnableInput (Game|GetPlayerController 0))
  (Input|EnableInput (Game|GetPlayerController 1))
  (Rendering|SetVisibility (Components|GetChildrenComponents (Variables|Default|GetPlayerSelect) false) false false)
  (Rendering|Components|Light|SetIntensity (Variables|Default|GetBlueSpotLight1) (Variables|Default|GetLightIntensity))
  (Variables|Default|SetP1Highlight 1)
  (Rendering|Components|Light|SetIntensity (Variables|Default|GetYellowSpotLight4) (Variables|Default|GetLightIntensity))
  (Variables|Default|SetP2Highlight 4))

(event Collision|EventActorBeginOverlap
  (params (OtherActor :type Actor%20Object%20Reference)))

(event EventTick
  (params (DeltaSeconds :type Float%20%28single-precision%29)))

(event Input|ActionEvents|InputActionCancel1
  (params (Key :type Key%20Structure))
  ;[0 0.1451 1] PLAYER 1
  ;;[1 1 1] PLAYER 1 CANCEL
  (:Pressed
    (Utilities|FlowControl|Sequence
      (:then_0
        (if (== (Variables|Default|GetP1Highlight) 1)
          (Rendering|Components|Light|SetLightColor (Variables|Default|GetBlueSpotLight1) "(R=0.356863,G=0.349020,B=1.000000,A=1.000000)" true)
          (Variables|Default|SetP1Validation false :!label _label)))
      (:then_1
        (if (== (Variables|Default|GetP1Highlight) 2)
          (Rendering|Components|Light|SetLightColor (Variables|Default|GetBlueSpotLight2) "(R=0.356863,G=0.349020,B=1.000000,A=1.000000)" true)
          (goto _label)))
      (:then_2
        (if (== (Variables|Default|GetP1Highlight) 3)
          (Rendering|Components|Light|SetLightColor (Variables|Default|GetBlueSpotLight3) "(R=0.356863,G=0.349020,B=1.000000,A=1.000000)" true)
          (goto _label)))
      (:then_3
        (if (== (Variables|Default|GetP1Highlight) 4)
          (Rendering|Components|Light|SetLightColor (Variables|Default|GetBlueSpotLight4) "(R=0.356863,G=0.349020,B=1.000000,A=1.000000)" true)
          (goto _label))))))

(fn ConstructionScript)
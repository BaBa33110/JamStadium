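; TempoLine_BP is a flipbook-based tempo line Blueprint for Jam Stadium.
; BeginPlay sets the flipbook to normal play rate, and a Loop event snaps it back to the first frame without firing events.
; Unconnected logic would tint the sprite green or white from the player controller's GlobalTiming flag, but it never runs.
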(event Custom|Loop
  (Class|PaperFlipbookComponent|SetPlaybackPositioninFrames (Variables|Default|GetFlipBook) 0 false))

(event EventBeginPlay
  (Components|Timeline|SetPlayRate (Variables|Default|GetFlipBook) 1.0))

(event Collision|EventActorBeginOverlap
  (params (OtherActor :type Actor%20Object%20Reference)))

(event EventTick
  (params (DeltaSeconds :type Float%20%28single-precision%29)))

(fn ConstructionScript)
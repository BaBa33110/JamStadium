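; Scoreboard actor for JamStadium that displays both players' scores as world-space text.
; ActualiseScore reads P1Score and P2Score from PlayerGameMode and writes them to TextRender1 and TextRender respectively.
; It runs on BeginPlay and does not poll on Tick, so any later refresh depends on the event being called again.
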(event Custom|ActualiseScore
  (bind _returnvalue (Game|GetGameMode))
  (bind _asplayer_game_mode (Utilities|Casting|CastToPlayerGameMode _returnvalue))
  (Rendering|Components|TextRender|SetText (Variables|Default|GetTextRender1) (Utilities|Text|ToText(Integer) (Variables|/Game/JamStadium/PlayerGameMode.PlayerGameMode_C|GetP1Score _asplayer_game_mode)))
  (Rendering|Components|TextRender|SetText (Variables|Default|GetTextRender) (Utilities|Text|ToText(Integer) (Variables|/Game/JamStadium/PlayerGameMode.PlayerGameMode_C|GetP2Score _asplayer_game_mode))))

(event EventBeginPlay
  (CallFunction|ActualiseScore))

(event Collision|EventActorBeginOverlap
  (params (OtherActor :type Actor%20Object%20Reference)))

(event EventTick
  (params (DeltaSeconds :type Float%20%28single-precision%29)))

(fn ConstructionScript)
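; Short-lived ultimate attack actor that hits a cross of five cases (centre, up, down, left, right) in Jam Stadium.
; On BeginPlay it removes arms whose case and trigger match hard-coded edge position ranges, spawns ExplosionHalo effects at all five case transforms, and self-destructs after a brief delay.
; Any trigger overlapping a Player-tagged component flags a critical in PlayerGameMode and calls NewRound with that component's location to zoom on.
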(event OnComponentBeginOverlap(MidTrigger)
  (params (OverlappedComponent :type Primitive%20Component%20Object%20Reference) (OtherActor :type Actor%20Object%20Reference) (OtherComp :type Primitive%20Component%20Object%20Reference) (OtherBodyIndex :type Integer) (bFromSweep :type Boolean) (SweepResult :type Hit%20Result%20Structure%20%28by%20ref%29))
  (bind _returnvalue (Game|GetGameMode))
  (bind _asplayer_game_mode (Utilities|Casting|CastToPlayerGameMode _returnvalue))
  (if (Components|ComponentHasTag OtherComp "Player")
    (Variables|/Game/JamStadium/PlayerGameMode.PlayerGameMode_C|SetIsCritical _asplayer_game_mode true)
    (Default|NewRound _asplayer_game_mode 0 (Transformation|GetWorldLocation OtherComp) OtherComp)))

(event OnComponentBeginOverlap(UpTrigger)
  (params (OverlappedComponent :type Primitive%20Component%20Object%20Reference) (OtherActor :type Actor%20Object%20Reference) (OtherComp :type Primitive%20Component%20Object%20Reference) (OtherBodyIndex :type Integer) (bFromSweep :type Boolean) (SweepResult :type Hit%20Result%20Structure%20%28by%20ref%29))
  (bind _returnvalue (Game|GetGameMode))
  (bind _asplayer_game_mode (Utilities|Casting|CastToPlayerGameMode _returnvalue))
  (if (Components|ComponentHasTag OtherComp "Player")
    (Variables|/Game/JamStadium/PlayerGameMode.PlayerGameMode_C|SetIsCritical _asplayer_game_mode true)
    (Default|NewRound _asplayer_game_mode 0 (Transformation|GetWorldLocation OtherComp) OtherComp)))

(event OnComponentBeginOverlap(DownTrigger)
  (params (OverlappedComponent :type Primitive%20Component%20Object%20Reference) (OtherActor :type Actor%20Object%20Reference) (OtherComp :type Primitive%20Component%20Object%20Reference) (OtherBodyIndex :type Integer) (bFromSweep :type Boolean) (SweepResult :type Hit%20Result%20Structure%20%28by%20ref%29))
  (bind _returnvalue (Game|GetGameMode))
  (bind _asplayer_game_mode (Utilities|Casting|CastToPlayerGameMode _returnvalue))
  (if (Components|ComponentHasTag OtherComp "Player")
    (Variables|/Game/JamStadium/PlayerGameMode.PlayerGameMode_C|SetIsCritical _asplayer_game_mode true)
    (Default|NewRound _asplayer_game_mode 0 (Transformation|GetWorldLocation OtherComp) OtherComp)))

(event OnComponentBeginOverlap(RightTrigger)
  (params (OverlappedComponent :type Primitive%20Component%20Object%20Reference) (OtherActor :type Actor%20Object%20Reference) (OtherComp :type Primitive%20Component%20Object%20Reference) (OtherBodyIndex :type Integer) (bFromSweep :type Boolean) (SweepResult :type Hit%20Result%20Structure%20%28by%20ref%29))
  (bind _returnvalue (Game|GetGameMode))
  (bind _asplayer_game_mode (Utilities|Casting|CastToPlayerGameMode _returnvalue))
  (if (Components|ComponentHasTag OtherComp "Player")
    (Variables|/Game/JamStadium/PlayerGameMode.PlayerGameMode_C|SetIsCritical _asplayer_game_mode true)
    (Default|NewRound _asplayer_game_mode 0 (Transformation|GetWorldLocation OtherComp) OtherComp)))

(event OnComponentBeginOverlap(LeftTrigger)
  (params (OverlappedComponent :type Primitive%20Component%20Object%20Reference) (OtherActor :type Actor%20Object%20Reference) (OtherComp :type Primitive%20Component%20Object%20Reference) (OtherBodyIndex :type Integer) (bFromSweep :type Boolean) (SweepResult :type Hit%20Result%20Structure%20%28by%20ref%29))
  (bind _returnvalue (Game|GetGameMode))
  (bind _asplayer_game_mode (Utilities|Casting|CastToPlayerGameMode _returnvalue))
  (if (Components|ComponentHasTag OtherComp "Player")
    (Variables|/Game/JamStadium/PlayerGameMode.PlayerGameMode_C|SetIsCritical _asplayer_game_mode true)
    (Default|NewRound _asplayer_game_mode 0 (Transformation|GetWorldLocation OtherComp) OtherComp)))

(event EventBeginPlay
  (Utilities|FlowControl|Sequence
    (:then_0
      (if (Math|Float|InRange(Float) (.y (Transformation|GetActorLocation)) -2.2e+02 -1.8e+02)
        (Components|DestroyComponent (Variables|Default|GetUpCase))))
    (:then_1
      (if (Math|Float|InRange(Float) (.y (Transformation|GetActorLocation)) -2e+01 2e+01)
        (Components|DestroyComponent (Variables|Default|GetDownCase))))
    (:then_2
      (if (Math|Float|InRange(Float) (.x (Transformation|GetActorLocation)) 2.8e+02 3.2e+02)
        (Components|DestroyComponent (Variables|Default|GetRightCase))))
    (:then_3
      (if (Math|Float|InRange(Float) (.x (Transformation|GetActorLocation)) -3.2e+02 -2.8e+02)
        (Components|DestroyComponent (Variables|Default|GetLeftCase))))
    (:then_4
      (Utilities|FlowControl|Delay 0.4)
      (Actor|DestroyActor))
    (:then_5
      (bind _returnvalue (Game|SpawnActorfromClass "/Game/JamStadium/ExplosionHalo.ExplosionHalo_C" (Transformation|GetWorldTransform (Variables|Default|GetUpCase)) "Undefined" 0 0))
      (Default|HaloEffect _returnvalue 1)
      (bind _returnvalue_2 (Game|SpawnActorfromClass "/Game/JamStadium/ExplosionHalo.ExplosionHalo_C" (Transformation|GetWorldTransform (Variables|Default|GetDownCase)) "Undefined" 0 0))
      (Default|HaloEffect _returnvalue_2 1)
      (bind _returnvalue_3 (Game|SpawnActorfromClass "/Game/JamStadium/ExplosionHalo.ExplosionHalo_C" (Transformation|GetWorldTransform (Variables|Default|GetLeftCase)) "Undefined" 0 0))
      (Default|HaloEffect _returnvalue_3 1)
      (bind _returnvalue_4 (Game|SpawnActorfromClass "/Game/JamStadium/ExplosionHalo.ExplosionHalo_C" (Transformation|GetWorldTransform (Variables|Default|GetRightCase)) "Undefined" 0 0))
      (Default|HaloEffect _returnvalue_4 1)
      (bind _returnvalue_5 (Game|SpawnActorfromClass "/Game/JamStadium/ExplosionHalo.ExplosionHalo_C" (Transformation|GetWorldTransform (Variables|Default|GetMidCase)) "Undefined" 0 0))
      (Default|HaloEffect _returnvalue_5 1))))

(event EventTick
  (params (DeltaSeconds :type Float%20%28single-precision%29)))

(fn ConstructionScript)
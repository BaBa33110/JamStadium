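; Animated stadium speaker prop in JamStadium, driven by custom events.
; Bump pulses the actor's scale with a timeline, while SpeakerGoUp and SpeakerGoDown use timelines to lerp it up by a small step or down to a fixed height.
; TwinkleSpeakers loops on delays, flashing three mesh parts pink and blue until StopTwinkling clears the flag and restores their original materials.
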(event Custom|Bump
  (bind _float (Timeline|ScalingTimeline PlayFromStart)
    (:Update
      (Transformation|SetActorScale3D (Math|Vector|Lerp(Vector) "1.600000,1.600000,1.600000" "1.700000,1.700000,1.650000" _float)))))

(event Custom|SpeakerGoDown
  (bind _returnvalue (Transformation|GetActorLocation))
  (bind _lerpfloat (Timeline|Timeline_0 PlayFromStart)
    (:Update
      (Transformation|SetActorLocation (Math|Vector|Lerp(Vector) (Transformation|GetActorLocation) (Math|Vector|MakeVector (.x _returnvalue) (.y _returnvalue) -1.2e+02) _lerpfloat) false false))))

(event Custom|StopTwinkling
  (Variables|Default|SetIsTwinkling false)
  (Rendering|Material|SetMaterial (Variables|Default|Gethifi_pPipe1) 0 "/Game/SceneTypeElements/Models/Speaker1/hangfalfelso.hangfalfelso")
  (Rendering|Material|SetMaterial (Variables|Default|Gethifi_pPipe2) 0 "/Game/SceneTypeElements/Models/Speaker1/hangfalaslo.hangfalaslo")
  (Rendering|Material|SetMaterial (Variables|Default|Gethifi_pCube2) 0 "/Game/SceneTypeElements/Models/Speaker1/közepdisz.közepdisz"))

(event Custom|TwinkleSpeakers
  (Variables|Default|SetIsTwinkling true)
  (if (Variables|Default|GetIsTwinkling) :!label _label
    (Rendering|Material|SetMaterial (Variables|Default|Gethifi_pPipe1) 0 "/Game/JamStadium/Graphics/Materials/Pink_Mat.Pink_Mat")
    (Utilities|FlowControl|Delay 0.15)
    (Rendering|Material|SetMaterial (Variables|Default|Gethifi_pPipe1) 0 "/Game/JamStadium/Graphics/Materials/Blue_Mat.Blue_Mat")
    (Utilities|FlowControl|Delay 0.15)
    (goto _label)))

(event Custom|SpeakerGoUp
  (bind _returnvalue (Transformation|GetActorLocation))
  (Variables|Default|SetLocation (Math|Vector|MakeVector (.x _returnvalue) (.y _returnvalue) (+ (.z _returnvalue) 8.0)))
  (bind _lerpfloat (Timeline|TimelineUp PlayFromStart)
    (:Update
      (Transformation|SetActorLocation (Math|Vector|Lerp(Vector) (Transformation|GetActorLocation) (Variables|Default|GetLocation) _lerpfloat) false false))))

(event EventBeginPlay)

(event Collision|EventActorBeginOverlap
  (params (OtherActor :type Actor%20Object%20Reference)))

(event EventTick
  (params (DeltaSeconds :type Float%20%28single-precision%29)))

(fn ConstructionScript)